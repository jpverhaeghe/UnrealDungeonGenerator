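; BP_LayoutGenerator procedurally generates a grid dungeon on BeginPlay, or at a random size through GenerateDungeon, and spawns it into the level.
; Starting from a random all-exit room, GenerateRoom recursively follows exits, re-rolling random room types until they fit grid edges and placed neighbours.
; Exit checks match substrings of enum names.
; The flat-array layout becomes scaled BP_Room actors with walls and optional lava, tracked for cleanup.
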(event EventBeginPlay
  ;[1 1 1] Create a dungeon of the size provided by the user and print it to the viewport
  (CallFunction|GenerateDungeonLayout (Variables|Default|GetMaxNumRooms_X) (Variables|Default|GetMaxNumRooms_Y))
  (CallFunction|PrintDungeon))

(fn ConstructionScript)

(fn GenerateDungeon
  ;[1 1 1] Randomize the dungeon size (will make UI elements)
  (CallFunction|GenerateDungeonLayout (Math|Random|RandomIntegerinRange 5 (Variables|Default|GetMaxNumRooms_X)) (Math|Random|RandomIntegerinRange 5 (Variables|Default|GetMaxNumRooms_Y)))
  (CallFunction|PrintDungeon))

(fn ClearDungeon
  (params (ArraySize :type Integer))
  (bind _dungeonlayout (Variables|Default|GetDungeonLayout))
  (bind _dungeonrooms (Variables|Default|GetDungeonRooms))
  ;[1 1 1] Clears the current dungeon by setting all elements to Clr (the 0th element)
  (for _array_element _dungeonrooms
    (Default|DestryoWalls _array_element)
    (Actor|DestroyActor _array_element))
  (Utilities|Array|Clear _dungeonrooms)
  (Utilities|Array|Clear _dungeonlayout)
  (for _index (range 0 (- ArraySize 1))
    (Utilities|Array|SetArrayElem _dungeonlayout _index "NewEnumerator0" true)))

(fn GenerateDungeonLayout
  (params (DungeonWidth :type Integer) (DungeonHeight :type Integer))
  ;[1 1 1] Compute dungeon array size and clear the dungeon array
  (bind _output_get (Variables|Default|SetDungeonLayoutHeight DungeonHeight))
  (bind _output_get_2 (Variables|Default|SetDungeonLayoutWidth DungeonWidth))
  (CallFunction|ClearDungeon (* DungeonWidth DungeonHeight))
  ;[1 1 1] Randomize the starting position in the array and set the first room to a NESW room
  (bind _output_get_3 (Variables|Default|SetStartRoomY (Math|Random|RandomIntegerinRange 1 (- _output_get 2))))
  (bind _output_get_4 (Variables|Default|SetStartRoomX (Math|Random|RandomIntegerinRange 1 (- _output_get_2 2))))
  (bind _arraypos (CallFunction|GetArrayPos _output_get_4 _output_get_3))
  (Utilities|Array|SetArrayElem (Variables|Default|GetDungeonLayout) _arraypos "NewEnumerator1")
  ;[1 1 1] If we are not at the top edge of the layout (y==0) then try to place a room North
  (if (== (Variables|Default|GetStartRoomY) 0)
    _
    (else
      (CallFunction|GenerateRoom "NewEnumerator2" (Variables|Default|GetStartRoomX) (- (Variables|Default|GetStartRoomY) 1))))
  ;[1 1 1] If we are not at the right edge of the layout (x==width) then try to place a room East
  (if (== (Variables|Default|GetStartRoomX) (- (Variables|Default|GetDungeonLayoutWidth) 1))
    _
    (else
      (CallFunction|GenerateRoom "NewEnumerator3" (+ (Variables|Default|GetStartRoomX) 1) (Variables|Default|GetStartRoomY))))
  ;[1 1 1] If we are not at the bottom edge of the layout (y==height -1) then try to place a room South
  (if (== (Variables|Default|GetStartRoomY) (- (Variables|Default|GetDungeonLayoutHeight) 1))
    _
    (else
      (CallFunction|GenerateRoom "NewEnumerator0" (Variables|Default|GetStartRoomX) (+ (Variables|Default|GetStartRoomY) 1))))
  ;[1 1 1] If we are not at the left edge of the layout (x==0) then try to place a room West
  (if (== (Variables|Default|GetStartRoomX) 0)
    _
    (else
      (CallFunction|GenerateRoom "NewEnumerator1" (- (Variables|Default|GetStartRoomX) 1) (Variables|Default|GetStartRoomY))))
  (return))

(fn GenerateRoom
  (params (ExitDirectionNeeded :type ExitDirection%20Enum :default "NewEnumerator0") (CurrentRoomPosX :type Integer) (CurrentRoomPosY :type Integer))
  ;[1 1 1] Get the current room type at this location in the dungeon layout (stored locally)
  (LocalVariables|SetcurrentRow CurrentRoomPosY)
  (LocalVariables|SetcurrentCol CurrentRoomPosX)
  (bind _arraypos (CallFunction|GetArrayPos CurrentRoomPosX CurrentRoomPosY))
  (bind _output_get (LocalVariables|SetcurrentArrayPos _arraypos))
  (bind _output_get_2 (LocalVariables|SetcurrentRoomType (Utilities|Array|Get(acopy) (Variables|Default|GetDungeonLayout) _output_get)))
  ;[1 1 1] Base condition for a room is if it has already been placed - not Clr
  (if (Utilities|Enum|Equal(Enum) _output_get_2 "NewEnumerator0")
    ;[1 1 1] Loop until we find a room that is available for this location (choosing a random room type each time)
    (while (not (Utilities|String|Contains (Utilities|String|EnumtoString (LocalVariables|GetcurrentRoomType)) (Utilities|String|EnumtoString ExitDirectionNeeded))) :!label _label
      (LocalVariables|SetcurrentRoomType (Utilities|Enum|ByteToEnumRoomType (Math|Conversions|ToByte(Integer) (Math|Random|RandomIntegerinRange 1 (- (|GetNumEnumEntries) 1)))))
      ;[1 1 1] If on an edge and room type has an exit that way, set the room to clear and try again
      (if (Math|Boolean|ORBoolean (and (Utilities|String|Contains (Utilities|String|EnumtoString (LocalVariables|GetcurrentRoomType)) (Utilities|String|EnumtoString (Utilities|Enum|LiteralenumExitDirection "NewEnumerator0"))) (== (LocalVariables|GetcurrentRow) 0)) (and (Utilities|String|Contains (Utilities|String|EnumtoString (LocalVariables|GetcurrentRoomType)) (Utilities|String|EnumtoString (Utilities|Enum|LiteralenumExitDirection "NewEnumerator1"))) (== (LocalVariables|GetcurrentCol) (- (Variables|Default|GetDungeonLayoutWidth) 1))) (and (Utilities|String|Contains (Utilities|String|EnumtoString (LocalVariables|GetcurrentRoomType)) (Utilities|String|EnumtoString (Utilities|Enum|LiteralenumExitDirection "NewEnumerator2"))) (== (LocalVariables|GetcurrentRow) (- (Variables|Default|GetDungeonLayoutHeight) 1))) (and (Utilities|String|Contains (Utilities|String|EnumtoString (LocalVariables|GetcurrentRoomType)) (Utilities|String|EnumtoString (Utilities|Enum|LiteralenumExitDirection "NewEnumerator3"))) (== (LocalVariables|GetcurrentCol) 0)))
        (LocalVariables|SetcurrentRoomType "NewEnumerator0")
        (goto _label)
        (else
          ;[1 1 1] Check surrounding rooms to see if they have exits that work with this room
          (bind _newroomtype (CallFunction|CheckSurroundingRooms (LocalVariables|GetcurrentRoomType) (LocalVariables|GetcurrentRow) (LocalVariables|GetcurrentCol)))
          (LocalVariables|SetcurrentRoomType _newroomtype)
          (goto _label))))
    ;[1 1 1] Set the new room to the array at the room pos
    (Utilities|Array|SetArrayElem (Variables|Default|GetDungeonLayout) (LocalVariables|GetcurrentArrayPos) (LocalVariables|GetcurrentRoomType))
    ;[1 1 1] If there is an exit north, follow that direction and generate rooms until there are no more
    (if (Utilities|String|Contains (Utilities|String|EnumtoString (LocalVariables|GetcurrentRoomType)) (Utilities|String|EnumtoString (Utilities|Enum|LiteralenumExitDirection "NewEnumerator0")))
      (CallFunction|GenerateRoom "NewEnumerator2" (LocalVariables|GetcurrentCol) (- (LocalVariables|GetcurrentRow) 1)))
    ;[1 1 1] If there is an exit east, follow that direction and generate rooms until there are no more
    (if (Utilities|String|Contains (Utilities|String|EnumtoString (LocalVariables|GetcurrentRoomType)) (Utilities|String|EnumtoString (Utilities|Enum|LiteralenumExitDirection "NewEnumerator1")))
      (CallFunction|GenerateRoom "NewEnumerator3" (+ (LocalVariables|GetcurrentCol) 1) (LocalVariables|GetcurrentRow)))
    ;[1 1 1] If there is an exit south, follow that direction and generate rooms until there are no more
    (if (Utilities|String|Contains (Utilities|String|EnumtoString (LocalVariables|GetcurrentRoomType)) (Utilities|String|EnumtoString (Utilities|Enum|LiteralenumExitDirection "NewEnumerator2")))
      (CallFunction|GenerateRoom "NewEnumerator0" (LocalVariables|GetcurrentCol) (+ (LocalVariables|GetcurrentRow) 1)))
    ;[1 1 1] If there is an exit west, follow that direction and generate rooms until there are no more
    (if (Utilities|String|Contains (Utilities|String|EnumtoString (LocalVariables|GetcurrentRoomType)) (Utilities|String|EnumtoString (Utilities|Enum|LiteralenumExitDirection "NewEnumerator3")))
      (CallFunction|GenerateRoom "NewEnumerator1" (- (LocalVariables|GetcurrentCol) 1) (LocalVariables|GetcurrentRow)))
    (return)))

(fn PrintDungeon
  (bind _dungeonlayoutwidth (Variables|Default|GetDungeonLayoutWidth))
  ;[1 1 1] Loop through each element in the dungeon layout
  (for _index (range 0 (- (Utilities|Array|Length (Variables|Default|GetDungeonLayout)) 1))
    ;[1 1 1] Calculate the row and column based off the width
    (bind _arraypos (CallFunction|GetArrayPos (Math|Integer|%(Integer) _index _dungeonlayoutwidth) (/ _index _dungeonlayoutwidth)))
    ;[1 1 1] If the room is not clear, print the room
    (if (not (Utilities|Enum|Equal(Enum) (Utilities|Array|Get(acopy) (Variables|Default|GetDungeonLayout) _arraypos) "NewEnumerator0"))
      (CallFunction|PrintRoom (Math|Integer|%(Integer) _index _dungeonlayoutwidth) (/ _index _dungeonlayoutwidth) (Utilities|Array|Get(acopy) (Variables|Default|GetDungeonLayout) _arraypos)))))

(fn PrintRoom
  (params (RoomPosX :type Integer) (RoomPosY :type Integer) (RoomType :type RoomType%20Enum :default "NewEnumerator0"))
  (bind _returnvalue (Math|Conversions|ToFloat(Integer) RoomPosY))
  (bind _returnvalue_2 (Math|Conversions|ToFloat(Integer) RoomPosX))
  (bind _roomsizex (Variables|Default|GetRoomSizeX))
  (bind _roomsizey (Variables|Default|GetRoomSizeY))
  (bind _returnvalue_3 (Math|Conversions|ToFloat(Integer) _roomsizex))
  (bind _returnvalue_4 (Math|Conversions|ToFloat(Integer) _roomsizey))
  (bind _returnvalue_5 (|((size*arrayPos)*100) _returnvalue_4 _returnvalue))
  (bind _returnvalue_6 (|((size*arrayPos)*100) _returnvalue_3 _returnvalue_2))
  (bind _returnvalue_7 (Math|Vector|MakeVector _returnvalue_6 _returnvalue_5 0.0))
  ;[1 1 1] Set variables for the new room, set the transform, spawn it and its walls, and add it to the room array for clean up later
  (bind _returnvalue_8 (Game|SpawnActorfromClass "/Game/MyBlueprints/BP_Room.BP_Room_C" (Math|Transform|MakeTransform _returnvalue_7 (Transformation|GetActorRotation) (Math|Vector|MakeVector (Math|Conversions|ToFloat(Integer) _roomsizex) (Math|Conversions|ToFloat(Integer) _roomsizey) 1.0)) "Undefined" 0 0))
  (Variables|/Game/MyBlueprints/BP_Room.BP_Room_C|SetWorldPos _returnvalue_8 _returnvalue_7)
  (Variables|/Game/MyBlueprints/BP_Room.BP_Room_C|SetDungeonPosX _returnvalue_8 _roomsizex)
  (Variables|/Game/MyBlueprints/BP_Room.BP_Room_C|SetDungeonPosY _returnvalue_8 _roomsizey)
  (Variables|/Game/MyBlueprints/BP_Room.BP_Room_C|SetRoomType _returnvalue_8 RoomType)
  (Default|SetLava _returnvalue_8 (Variables|Default|GetLavaRooms) (Variables|Default|GetLavaPercent))
  (Default|DrawWalls _returnvalue_8 (Variables|Default|GetWallMaterial))
  (Utilities|Array|Add (Variables|Default|GetDungeonRooms) _returnvalue_8))

(fn GetArrayPos
  (params (xPos :type Integer) (yPos :type Integer))
  ;[1 1 1] Using a single array so finding an index will use (y * Width) + x
  (return (Math|Float|Truncate (|((y*width)+x) (Math|Conversions|ToFloat(Integer) yPos) (Math|Conversions|ToFloat(Integer) (Variables|Default|GetDungeonLayoutWidth)) (Math|Conversions|ToFloat(Integer) xPos)))))

(fn CheckSurroundingRooms
  (params (currentRoomType :type RoomType%20Enum :default "NewEnumerator0") (currentRow :type Integer) (currentCol :type Integer))
  ;[1 1 1] Store local variables
  (LocalVariables|SetroomType currentRoomType)
  (LocalVariables|Setrow currentRow)
  (LocalVariables|Setcol currentCol)
  ;[1 1 1] Check North exit room
  (if (> (LocalVariables|Getrow) 0)
    (bind _arraypos (CallFunction|GetArrayPos (LocalVariables|Getcol) (- (LocalVariables|Getrow) 1)))
    (bind _roomtypeout (CallFunction|CheckRoomConnection (LocalVariables|GetroomType) (Utilities|Array|Get(acopy) (Variables|Default|GetDungeonLayout) _arraypos) "NewEnumerator0" "NewEnumerator2"))
    (if (Utilities|Enum|Equal(Enum) _roomtypeout "NewEnumerator0")
      (LocalVariables|SetroomType _roomtypeout)
      (else
        ;[1 1 1] Check South exit room
        (if (< (LocalVariables|Getrow) (- (Variables|Default|GetDungeonLayoutHeight) 1)) :!label _label
          (bind _arraypos_2 (CallFunction|GetArrayPos (LocalVariables|Getcol) (+ (LocalVariables|Getrow) 1)))
          (bind _roomtypeout_2 (CallFunction|CheckRoomConnection (LocalVariables|GetroomType) (Utilities|Array|Get(acopy) (Variables|Default|GetDungeonLayout) _arraypos_2) "NewEnumerator2" "NewEnumerator0"))
          (if (Utilities|Enum|Equal(Enum) _roomtypeout_2 "NewEnumerator0")
            (LocalVariables|SetroomType _roomtypeout_2)
            (else
              ;[1 1 1] Check West exit room
              (if (> (LocalVariables|Getcol) 0) :!label _label_2
                (bind _arraypos_3 (CallFunction|GetArrayPos (- (LocalVariables|Getcol) 1) (LocalVariables|Getrow)))
                (bind _roomtypeout_3 (CallFunction|CheckRoomConnection (LocalVariables|GetroomType) (Utilities|Array|Get(acopy) (Variables|Default|GetDungeonLayout) _arraypos_3) "NewEnumerator3" "NewEnumerator1"))
                (if (Utilities|Enum|Equal(Enum) _roomtypeout_3 "NewEnumerator0")
                  (LocalVariables|SetroomType _roomtypeout_3)
                  (else
                    ;[1 1 1] Check East exit room
                    (if (< (LocalVariables|Getcol) (- (Variables|Default|GetDungeonLayoutWidth) 1)) :!label _label_3
                      (bind _arraypos_4 (CallFunction|GetArrayPos (+ (LocalVariables|Getcol) 1) (LocalVariables|Getrow)))
                      (bind _roomtypeout_4 (CallFunction|CheckRoomConnection (LocalVariables|GetroomType) (Utilities|Array|Get(acopy) (Variables|Default|GetDungeonLayout) _arraypos_4) "NewEnumerator1" "NewEnumerator3"))
                      (if (Utilities|Enum|Equal(Enum) _roomtypeout_4 "NewEnumerator0")
                        (LocalVariables|SetroomType _roomtypeout_4)))))
                (else
                  (goto _label_3)))))
          (else
            (goto _label_2)))))
    (else
      (goto _label)))
  (return (LocalVariables|GetroomType)))

(fn CheckRoomConnection
  (params (currentRoom :type RoomType%20Enum :default "NewEnumerator0") (compareRoom :type RoomType%20Enum :default "NewEnumerator0") (currentExit :type ExitDirection%20Enum :default "NewEnumerator0") (compareExit :type ExitDirection%20Enum :default "NewEnumerator0"))
  ;[1 1 1] Set up the check, if the room is a clr room, then just exit with that value
  (LocalVariables|SetroomTypeUpdated currentRoom)
  (if (Utilities|Enum|Equal(Enum) compareRoom "NewEnumerator0")
    _
    (else
      ;[1 1 1] If the compare room has an exit in the direction we came, check the current room
      (if (Utilities|String|Contains (Utilities|String|EnumtoString compareRoom) (Utilities|String|EnumtoString compareExit))
        ;[1 1 1] Since the compare room has an exit towards our room, make sure we have one going that way or make reset tto a clear room
        (if (Utilities|String|Contains (Utilities|String|EnumtoString currentRoom) (Utilities|String|EnumtoString currentExit))
          _
          (else
            (LocalVariables|SetroomTypeUpdated "NewEnumerator0")))
        (else
          ;[1 1 1] If there is no exit in the compare room towards this room, and there is one going towards the compare room, then clear this room
          (if (Utilities|String|Contains (Utilities|String|EnumtoString currentRoom) (Utilities|String|EnumtoString currentExit))
            (LocalVariables|SetroomTypeUpdated "NewEnumerator0"))))))
  ;[1 1 1] Return the updated room
  (return (LocalVariables|GetroomTypeUpdated)))